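; Base enemy character that rewinds along with the player and supplies attack, patrol and movement functions.
; Each Tick it records transform and rotation in an unbounded history array, then pops and reapplies entries in reverse while the player's IsRewinding flag is set.
; Attack plays a melee montage and calls OnAttackEnd on completion or interruption.
; Helper functions expose ideal combat ranges and patrol route, and map speed states to walk speed.
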(event Custom|Attack
  (Animation|Montage|PlayMontage (Variables|Character|GetMesh) "/Game/_Custom/Enemy_Assets/Animation/Primary_Melee_D_Slow_Montage1.Primary_Melee_D_Slow_Montage1"
    (:then
      (Development|PrintString "attack end"))
    (:OnCompleted
      (Default|CallOnAttackEnd :!label _label))
    (:OnInterrupted
      (goto _label))))

(event EventTick
  (params (DeltaSeconds :type Float%20%28single-precision%29))
  (bind _characterdate (Variables|Default|GetCharacterDate))
  (bind _characterdate_2 (Variables|Default|GetCharacterDate))
  (bind _returnvalue (Utilities|Array|Length _characterdate_2))
  (bind _returnvalue_2 (- _returnvalue 1))
  (bind _output (Utilities|Array|Get(acopy) _characterdate_2 _returnvalue_2))
  (if (Variables|/Game/_Custom/Player_Assets/BP_ThirdPersonCharacter.BP_ThirdPersonCharacter_C|GetIsRewinding (Variables|Default|GetAs%20BP%20Third%20Person%20Character))
    (if (not (== (Utilities|Array|Length (Variables|Default|GetCharacterDate)) 0))
      (Transformation|SetActorTransform (.transform _output) true)
      (Transformation|SetActorRotation (.controlrotation _output))
      (Utilities|Array|RemoveIndex _characterdate (- (Utilities|Array|Length _characterdate) 1)))
    (else
      (Utilities|Array|Add (Variables|Default|GetCharacterDate) (Utilities|Struct|MakeCharacterFrameData (Transformation|GetActorTransform) (Transformation|GetActorRotation))))))

(event EventBeginPlay
  (bind _asbp_third_person_character (Utilities|Casting|CastToBP_ThirdPersonCharacter (Game|GetPlayerCharacter 0)))
  (Variables|Default|SetAs%20BP%20Third%20Person%20Character _asbp_third_person_character))

(fn ConstructionScript)

(fn GetIdealRange
  (return 1.5e+02 3.5e+02))

(fn GetPatrolRoute
  (return (Variables|Default|GetPatrolRoute)))

(fn SetMovementSpeed
  (params (Speed :type E_MovementSpeed%20Enum :default "NewEnumerator0"))
  (bind _output_get (Variables|/Script/Engine.CharacterMovementComponent|SetMaxWalkSpeed (Variables|Character|GetCharacterMovement) (Utilities|Select :Index Speed :NewEnumerator0 0.0 :NewEnumerator1 1e+02 :NewEnumerator2 3e+02 :NewEnumerator3 5e+02)))
  (return _output_get))