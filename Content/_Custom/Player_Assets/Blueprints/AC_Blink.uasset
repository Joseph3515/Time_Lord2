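; AC_Blink is an actor component that gives its owning Character a short forward blink.
; BeginPlay caches the owner as a Character for the Blink_Start event to use.
; Blink_Start spawns Niagara start and middle effects at the capsule and intended destination, then after a brief delay moves the capsule forward by BlinkDis with sweep.
; It then spawns the end effect at the resulting location and deactivates the middle effect.
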(event Custom|Blink_Start
  (bind _as_character (Variables|Default|GetAs%20Character))
  (bind _blink_dis (Variables|Default|GetBlink%20Dis))
  (bind _capsulecomponent (Variables|/Script/Engine.Character|GetCapsuleComponent _as_character))
  (bind _returnvalue (Math|Vector|GetForwardVector _capsulecomponent))
  (bind _returnvalue_2 (Transformation|GetWorldLocation _capsulecomponent))
  (bind _returnvalue_3 (* _returnvalue _blink_dis))
  (bind _returnvalue_4 (+ _returnvalue_2 _returnvalue_3))
  (Niagara|SpawnSystematLocation "/Game/_Custom/Player_Assets/Effects/NS_Start_Blink.NS_Start_Blink" _returnvalue_2)
  (bind _returnvalue_5 (Niagara|SpawnSystematLocation "/Game/_Custom/Player_Assets/Effects/NS_Middle_Blink.NS_Middle_Blink" _returnvalue_4))
  (Variables|Default|SetNs%20Middle%20Ref _returnvalue_5)
  (Utilities|FlowControl|Delay 0.2)
  (Transformation|SetWorldLocation _capsulecomponent _returnvalue_4 true false)
  (Niagara|SpawnSystematLocation "/Game/_Custom/Player_Assets/Effects/NS_End_Blink1.NS_End_Blink1" (Transformation|GetWorldLocation (Variables|/Script/Engine.Character|GetCapsuleComponent (Variables|Default|GetAs%20Character))))
  (Components|Activation|Deactivate (Variables|Default|GetNs%20Middle%20Ref)))

(event EventBeginPlay
  (Utilities|FlowControl|Sequence
    (:then_0
      (bind _ascharacter (Utilities|Casting|CastToCharacter (Components|GetOwner)))
      (Variables|Default|SetAs%20Character _ascharacter))))

(event EventTick
  (params (DeltaSeconds :type Float%20%28single-precision%29)))