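; Character component for a directional blink dash chosen by held WASD keys.
; BlinkTrace checks sphere path, ground line and capsule fit, shortening the distance by about one capsule width per failure.
; BlinkStart recomputes the destination (only forward uses the shortened distance), hides the mesh, disables input and spawns Niagara effects.
; After a time-dilation-scaled delay, EndBlink sweeps the capsule there and restores visibility, input and distance.
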(event Custom|Blink%20Start
  (bind _as_character (Variables|Default|GetAs%20Character))
  (bind _as_character_2 (Variables|Default|GetAs%20Character))
  (bind _as_character_3 (Variables|Default|GetAs%20Character))
  (bind _as_character_4 (Variables|Default|GetAs%20Character))
  (bind _capsulecomponent (Variables|/Script/Engine.Character|GetCapsuleComponent _as_character_2))
  (bind _capsulecomponent_2 (Variables|/Script/Engine.Character|GetCapsuleComponent _as_character))
  (bind _capsulecomponent_3 (Variables|/Script/Engine.Character|GetCapsuleComponent _as_character_3))
  (bind _capsulecomponent_4 (Variables|/Script/Engine.Character|GetCapsuleComponent _as_character_4))
  (bind _returnvalue (Transformation|GetWorldLocation _capsulecomponent))
  (bind _returnvalue_2 (Transformation|GetWorldLocation _capsulecomponent_2))
  (bind _returnvalue_3 (Transformation|GetWorldLocation _capsulecomponent_4))
  (bind _returnvalue_4 (Transformation|GetWorldLocation _capsulecomponent_3))
  (Utilities|FlowControl|Sequence
    (:then_0
      (Utilities|InputBlinkDirection :!label _label
        (:Forward
          ;[1 1 1] Blink Forward/BackWard Start Up- This sets up the distance of the Character future position when blinking
          (Rendering|SetVisibility (Variables|Default|GetMesh) false true)
          (Input|DisableInput (Variables|Default|GetAs%20Character) (Game|GetPlayerController 0))
          (Variables|Direction|SetWorld%20Location _returnvalue_3)
          (Variables|Direction|SetBlink%20Location (+ _returnvalue_3 (* (Math|Vector|GetForwardVector _capsulecomponent_4) (Variables|Direction|GetTemp%20Blink%20Distance))))
          ;[1 1 1] Blink In Between Effect- This is where to add future abilites or effects in between the blinks of each direction
          (bind _returnvalue_5 (Niagara|SpawnSystematLocation "/Game/_Custom/Player_Assets/Effects/NS_Start_Blink.NS_Start_Blink" (Variables|Direction|GetWorld%20Location)))
          (Variables|Default|SetStart%20Ref _returnvalue_5)
          (bind _returnvalue_6 (Niagara|SpawnSystematLocation "/Game/_Custom/Player_Assets/Effects/NS_Middle_Blink.NS_Middle_Blink" (Variables|Direction|GetBlink%20Location)))
          (Variables|Default|SetMiddle%20Ref _returnvalue_6)
          (bind _returnvalue_7 (Utilities|Time|SetTimerbyEvent (delegate Custom|End%20Blink) (* (Variables|Blink|GetBlink%20Delay) (Class|GameplayStatics|GetGlobalTimeDilation))))
          (Variables|Blink|SetBlink%20Timer _returnvalue_7))
        (:Backward
          (Rendering|SetVisibility (Variables|Default|GetMesh) false true)
          (Input|DisableInput (Variables|Default|GetAs%20Character) (Game|GetPlayerController 0))
          (Variables|Direction|SetWorld%20Location _returnvalue_4)
          (Variables|Direction|SetBlink%20Location (+ _returnvalue_4 (* (Math|Vector|GetForwardVector _capsulecomponent_3) (Variables|Direction|GetBlink%20Distance))))
          (Niagara|SpawnSystematLocation "/Game/_Custom/Player_Assets/Effects/NS_Start_Blink.NS_Start_Blink" (Variables|Direction|GetWorld%20Location))
          (bind _returnvalue_8 (Niagara|SpawnSystematLocation "/Game/_Custom/Player_Assets/Effects/NS_Middle_Blink.NS_Middle_Blink" (Variables|Direction|GetBlink%20Location)))
          (Variables|Default|SetMiddle%20Ref _returnvalue_8)
          (bind _returnvalue_9 (Utilities|Time|SetTimerbyEvent (delegate Custom|End%20Blink) (* (Variables|Blink|GetBlink%20Delay) (Class|GameplayStatics|GetGlobalTimeDilation))))
          (Variables|Blink|SetBlink%20Timer _returnvalue_9))
        (:Right
          ;[1 1 1] Blink Right/Left Start Up- This sets up the distance of the Character future position when blinking
          (Rendering|SetVisibility (Variables|Default|GetMesh) false true)
          (Input|DisableInput (Variables|Default|GetAs%20Character) (Game|GetPlayerController 0))
          (Variables|Direction|SetWorld%20Location _returnvalue_2)
          (Variables|Direction|SetBlink%20Location (+ _returnvalue_2 (* (Math|Vector|GetRightVector _capsulecomponent_2) (Variables|Direction|GetBlink%20Distance))))
          (Niagara|SpawnSystematLocation "/Game/_Custom/Player_Assets/Effects/NS_Start_Blink.NS_Start_Blink" (Variables|Direction|GetWorld%20Location))
          (bind _returnvalue_10 (Niagara|SpawnSystematLocation "/Game/_Custom/Player_Assets/Effects/NS_Middle_Blink.NS_Middle_Blink" (Variables|Direction|GetBlink%20Location)))
          (Variables|Default|SetMiddle%20Ref _returnvalue_10)
          (bind _returnvalue_11 (Utilities|Time|SetTimerbyEvent (delegate Custom|End%20Blink) (* (Variables|Blink|GetBlink%20Delay) (Class|GameplayStatics|GetGlobalTimeDilation))))
          (Variables|Blink|SetBlink%20Timer _returnvalue_11))
        (:Left
          (Rendering|SetVisibility (Variables|Default|GetMesh) false true)
          (Input|DisableInput (Variables|Default|GetAs%20Character) (Game|GetPlayerController 0))
          (Variables|Direction|SetWorld%20Location _returnvalue)
          (Variables|Direction|SetBlink%20Location (+ _returnvalue (* (Math|Vector|GetRightVector _capsulecomponent) (Variables|Direction|GetBlink%20Distance))))
          (Niagara|SpawnSystematLocation "/Game/_Custom/Player_Assets/Effects/NS_Start_Blink.NS_Start_Blink" (Variables|Direction|GetWorld%20Location))
          (bind _returnvalue_12 (Niagara|SpawnSystematLocation "/Game/_Custom/Player_Assets/Effects/NS_Middle_Blink.NS_Middle_Blink" (Variables|Direction|GetBlink%20Location)))
          (Variables|Default|SetMiddle%20Ref _returnvalue_12)
          (bind _returnvalue_13 (Utilities|Time|SetTimerbyEvent (delegate Custom|End%20Blink) (* (Variables|Blink|GetBlink%20Delay) (Class|GameplayStatics|GetGlobalTimeDilation))))
          (Variables|Blink|SetBlink%20Timer _returnvalue_13))))
    (:then_1
      (goto _label S))
    (:then_2
      (goto _label D))
    (:then_3
      (goto _label A))))

(event Custom|Blink%20Trace
  (bind (_world_location _forward_vec _right_vec) (CallFunction|DirectionVectors))
  (bind (_world_location_2 _forward_vec_2) (CallFunction|DirectionVectors))
  (Utilities|FlowControl|ForLoopwithBreak 0 (Variables|Default|GetLast%20Index)
    (:LoopBody
      (Utilities|FlowControl|Sequence
        (:then_0
          (Utilities|InputBlinkDirection :!label _label
            (:Forward
              (bind (_outhit _returnvalue) (Collision|SphereTraceByChannel (+ _world_location_2 "0.000000,0.000000,40.000000") (+ _world_location_2 _forward_vec_2) 2e+01 "TraceTypeQuery1" false 0 (Variables|Default|GetDraw%20Debug%20Type) :!label _label_2))
              (if _returnvalue
                (Utilities|UpDateTempBlinkDistance)
                (else
                  (bind (_outhit_2 _returnvalue_2) (Collision|LineTraceByChannel (+ (.TraceEnd (Collision|BreakHitResult _outhit)) "0.000000,0.000000,200.000000") (+ (.TraceEnd (Collision|BreakHitResult _outhit)) "0.000000,0.000000,-500.000000") "TraceTypeQuery1" false 0 (Variables|Default|GetDraw%20Debug%20Type)))
                  (if _returnvalue_2
                    (bind (_outhit_3 _returnvalue_3) (Collision|CapsuleTraceByChannel (+ (.Location (Collision|BreakHitResult _outhit_2)) (* (.Normal (Collision|BreakHitResult _outhit_2)) 1e+02)) (+ (.Location (Collision|BreakHitResult _outhit_2)) (* (.Normal (Collision|BreakHitResult _outhit_2)) 1e+02)) (* (Variables|Blink|GetDefaultOut%20Radius) 1.2) (Variables|Blink|GetDefault%20Out%20Half%20Height) "TraceTypeQuery1" false 0 (Variables|Default|GetDraw%20Debug%20Type)))
                    (if _returnvalue_3
                      (Utilities|UpDateTempBlinkDistance)
                      (else
                        (Variables|Direction|SetBlink%20Location (.TraceEnd (Collision|BreakHitResult _outhit_3)))
                        (CallFunction|BreakLoop)))
                    (else
                      (Utilities|UpDateTempBlinkDistance))))))
            (:Backward
              (goto _label_2))
            (:Right
              (bind (_outhit_4 _returnvalue_4) (Collision|SphereTraceByChannel (+ _world_location "0.000000,0.000000,20.000000") (+ _world_location _right_vec) 2e+01 "TraceTypeQuery1" false 0 (Variables|Default|GetDraw%20Debug%20Type) :!label _label_3))
              (if _returnvalue_4
                (Utilities|UpDateTempBlinkDistance)
                (else
                  (bind (_outhit_5 _returnvalue_5) (Collision|LineTraceByChannel (+ (.TraceEnd (Collision|BreakHitResult _outhit_4)) "0.000000,0.000000,100.000000") (+ (.TraceEnd (Collision|BreakHitResult _outhit_4)) "0.000000,0.000000,-500.000000") "TraceTypeQuery1" false 0 (Variables|Default|GetDraw%20Debug%20Type)))
                  (if _returnvalue_5
                    (bind (_outhit_6 _returnvalue_6) (Collision|CapsuleTraceByChannel (+ (.Location (Collision|BreakHitResult _outhit_5)) (* (.Normal (Collision|BreakHitResult _outhit_5)) 1e+02)) (+ (.Location (Collision|BreakHitResult _outhit_5)) (* (.Normal (Collision|BreakHitResult _outhit_5)) 1e+02)) (* (Variables|Blink|GetDefaultOut%20Radius) 1.2) (Variables|Blink|GetDefault%20Out%20Half%20Height) "TraceTypeQuery1" false 0 (Variables|Default|GetDraw%20Debug%20Type)))
                    (if _returnvalue_6
                      (Utilities|UpDateTempBlinkDistance)
                      (else
                        (Variables|Direction|SetBlink%20Location (.TraceEnd (Collision|BreakHitResult _outhit_6)))
                        (CallFunction|BreakLoop)))
                    (else
                      (Utilities|UpDateTempBlinkDistance))))))
            (:Left
              (goto _label_3))))
        (:then_1
          (goto _label S))
        (:then_2
          (goto _label D))
        (:then_3
          (goto _label A))))
    (:Completed
      (if (not (Variables|Blink|GetIsBlinking?))
        (Variables|Direction|SetBlink%20Location (.World%20Location (CallFunction|DirectionVectors)))
        (Variables|Blink|SetIsBlinking? true)
        (CallFunction|BlinkStart)))))

(event Custom|End%20Blink
  ;[1 1 1] Blink Ending- This finishes the Blink and sets location of the Forward/back and Right/Left Blinks
  (Transformation|SetWorldLocation (Variables|/Script/Engine.Character|GetCapsuleComponent (Variables|Default|GetAs%20Character)) (Variables|Direction|GetBlink%20Location) true false)
  (bind _returnvalue (Niagara|SpawnSystematLocation "/Game/_Custom/Player_Assets/Effects/NS_End_Blink1.NS_End_Blink1" (.World%20Location (CallFunction|DirectionVectors))))
  (Variables|Default|SetEnd%20Ref _returnvalue)
  ;[1 1 1] Post Blink- This Wraps up the blink and re-enable the player to Blink again
  (Components|Activation|Deactivate (Variables|Default|GetMiddle%20Ref))
  (Rendering|SetVisibility (Variables|Default|GetMesh) true true)
  (Input|EnableInput (Variables|Default|GetAs%20Character) (Game|GetPlayerController 0))
  (Variables|Blink|SetIsBlinking? false)
  (Variables|Direction|SetTemp%20Blink%20Distance (Variables|Direction|GetBlink%20Distance)))

(event Custom|Break%20Loop
  (bind (_world_location _forward_vec _right_vec) (CallFunction|DirectionVectors))
  (bind (_world_location_2 _forward_vec_2) (CallFunction|DirectionVectors))
  (if (not (Variables|Blink|GetIsBlinking?))
    (Variables|Blink|SetIsBlinking? true)
    (CallFunction|BlinkStart)
    (Utilities|FlowControl|ForLoopwithBreak 0 (Variables|Default|GetLast%20Index)) ; enters at Break
  ))

(event EventBeginPlay
  (bind _ascharacter (Utilities|Casting|CastToCharacter (Components|GetOwner)))
  (Variables|Default|SetAs%20Character _ascharacter)
  (Variables|Default|SetMesh (Variables|/Script/Engine.Character|GetMesh _ascharacter))
  (Variables|Blink|SetDefaultOut%20Radius (.OutRadius (Components|Capsule|GetScaledCapsuleSize (Variables|/Script/Engine.Character|GetCapsuleComponent _ascharacter))))
  (Variables|Blink|SetDefault%20Out%20Half%20Height (.OutHalfHeight (Components|Capsule|GetScaledCapsuleSize (Variables|/Script/Engine.Character|GetCapsuleComponent _ascharacter))))
  (CallFunction|UpDateBlinkValue (Variables|Direction|GetBlink%20Distance)))

(fn Capsule/CharacterRef
  (bind _as_character (Variables|Default|GetAs%20Character))
  (return (Variables|/Script/Engine.Character|GetCapsuleComponent _as_character) (Variables|/Script/Engine.Character|GetCharacterMovement _as_character)))

(fn DirectionVectors
  (bind _capsulecomponent (CallFunction|Capsule/CharacterRef))
  (bind _temp_blink_distance (Variables|Direction|GetTemp%20Blink%20Distance))
  (return (Transformation|GetWorldLocation _capsulecomponent) (* (Math|Vector|Normalize (Math|Vector|GetForwardVector _capsulecomponent)) _temp_blink_distance) (* (Math|Vector|Normalize (Math|Vector|GetRightVector _capsulecomponent)) _temp_blink_distance)))

(fn UpDateBlinkValue
  (params (Temp%20Blink%20Distance :type Float%20%28single-precision%29))
  (Variables|Direction|SetTemp%20Blink%20Distance Temp%20Blink%20Distance)
  (Variables|Default|SetLast%20Index (Math|Float|Truncate (/ Temp%20Blink%20Distance (CallFunction|DimeterOfCapsule)))))

(fn DimeterOfCapsule
  (return (* (Variables|Blink|GetDefaultOut%20Radius) 2.4)))